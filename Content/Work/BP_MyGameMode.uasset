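; BP_MyGameMode is a game mode Blueprint that handles the end of a match through OnVictory and OnDefeat events.
; Each event lazily creates and caches its victory or defeat widget, then removes the referenced HUD via RemoveHUD.
; It then shows the mouse cursor, switches player 0 to UI-only input focused on that widget, adds it to the viewport and pauses the game.
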(event EventBeginPlay)

(event EventTick
  (params (DeltaSeconds :type Float%20%28single-precision%29)))

(event EventOnVictory
  (bind _returnvalue (Game|GetPlayerController 0))
  (Utilities|IsValid (Variables|Default|GetMy%20Victory%20UI%20Reference)
    (:Is%20Valid
      _)
    (:Is%20Not%20Valid
      (bind _returnvalue_2 (UserInterface|CreateWidget "/Game/Work/WBP_MyVictoryUI.WBP_MyVictoryUI_C"))
      (Variables|Default|SetMy%20Victory%20UI%20Reference _returnvalue_2)))
  (CallFunction|RemoveHUD)
  (Variables|/Script/Engine.PlayerController|SetbShowMouseCursor _returnvalue true)
  (Input|SetInputModeUIOnly _returnvalue (Variables|Default|GetMy%20Victory%20UI%20Reference) "DoNotLock")
  (UserInterface|Viewport|AddtoViewport (Variables|Default|GetMy%20Victory%20UI%20Reference) 0)
  (Game|SetGamePaused true))

(event EventOnDefeat
  (bind _returnvalue (Game|GetPlayerController 0))
  (Utilities|IsValid (Variables|Default|GetMy%20Defeat%20UI%20Reference)
    (:Is%20Valid
      _)
    (:Is%20Not%20Valid
      (bind _returnvalue_2 (UserInterface|CreateWidget "/Game/Work/WBP_MyDefeatUI.WBP_MyDefeatUI_C"))
      (Variables|Default|SetMy%20Defeat%20UI%20Reference _returnvalue_2)))
  (CallFunction|RemoveHUD)
  (Variables|/Script/Engine.PlayerController|SetbShowMouseCursor _returnvalue true)
  (Input|SetInputModeUIOnly _returnvalue (Variables|Default|GetMy%20Defeat%20UI%20Reference) "DoNotLock")
  (UserInterface|Viewport|AddtoViewport (Variables|Default|GetMy%20Defeat%20UI%20Reference) 0)
  (Game|SetGamePaused true))

(fn ConstructionScript)

(fn RemoveHUD
  (Widget|RemovefromParent (Variables|Default|GetHUD%20Reference)))