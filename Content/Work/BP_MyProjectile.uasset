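; BP_MyProjectile is a projectile Blueprint that keeps a live count of bullets in the world.
; BeginPlay increments AmountOfBulletReference on BP_MyGameMode, and Destroyed decrements it, each after casting the current game mode.
; The construction script only calls its parent, and the overlap and Tick events are unused.
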(event EventBeginPlay
  (bind _asbp_my_game_mode (Utilities|Casting|CastToBP_MyGameMode (Game|GetGameMode)))
  (Variables|/Script/Homework01.MyGameMode|SetAmountOfBulletReference _asbp_my_game_mode (+ (Variables|/Script/Homework01.MyGameMode|GetAmountOfBulletReference _asbp_my_game_mode) 1)))

(event Collision|EventActorBeginOverlap
  (params (OtherActor :type Actor%20Object%20Reference)))

(event EventTick
  (params (DeltaSeconds :type Float%20%28single-precision%29)))

(event EventDestroyed
  (bind _asbp_my_game_mode (Utilities|Casting|CastToBP_MyGameMode (Game|GetGameMode)))
  (Variables|/Script/Homework01.MyGameMode|SetAmountOfBulletReference _asbp_my_game_mode (- (Variables|/Script/Homework01.MyGameMode|GetAmountOfBulletReference _asbp_my_game_mode) 1)))

(fn ConstructionScript
  (|CallParentFunction))